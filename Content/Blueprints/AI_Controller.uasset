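; AI controller that runs a behavior tree targeting the player.
; On begin play it waits a short delay, starts AI_BehaviorTree, then finds the Player_BP actor and writes it to the blackboard's Target key.
; Tick is empty, and an unconnected cast to AI_pawn for its AiTarget never runs.
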(event `self.ReceiveBeginPlay`
  (`KismetSystemLibrary.Delay` 1.0)
  (`self.RunBehaviorTree` "/Game/Blueprints/AI_BehaviorTree.AI_BehaviorTree")
  (bind _returnvalue (`GameplayStatics.GetActorOfClass` "/Game/other/FirstPersonBP/Blueprints/Player_BP.Player_BP_C"))
  (set `self.Player` _returnvalue)
  (`BlackboardComponent.SetValueAsObject` (`AIBlueprintHelperLibrary.GetBlackboard` self) (`self.Target`) (`self.Player`)))

(event `self.ReceiveTick`
  (params (DeltaSeconds :type "Float (single-precision)")))

(fn `UserConstructionScript`)