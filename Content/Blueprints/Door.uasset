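; Destructible door actor that AI pawns damage or repair on contact, using hit points reset to maximum at BeginPlay.
; Overlapping pawns with the EnemyObject interface are destroyed: enemies subtract a hit point, builders add one, as does BuildWall.
; SetDoorState hides a staged mesh at low health and shows all meshes at other nonzero values.
; At zero it flags the door Dead, exposed through RemoveMe, and tells AIGoalManager to update goals.
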(event `self.ReceiveBeginPlay`
  (`SceneComponent.SetVisibility` (`self.StaticMesh1`) true false)
  (`SceneComponent.SetVisibility` (`self.StaticMesh2`) true false)
  (`SceneComponent.SetVisibility` (`self.StaticMesh3`) true false)
  (`SceneComponent.SetVisibility` (`self.StaticMesh`) true false)
  (set `self.HitPoints` (`self.MaxHitpoints`))
  (`SceneComponent.SetVisibility` (`self.StaticMesh`) true false))

(event `self.Sphere.OnComponentBeginOverlap`
  (params (OverlappedComponent :type "PrimitiveComponent Object Reference") (OtherActor :type "Actor Object Reference") (OtherComp :type "PrimitiveComponent Object Reference") (OtherBodyIndex :type Integer) (bFromSweep :type Boolean) (SweepResult :type "HitResult Structure (by ref)"))
  (bind _hitpoints (`self.HitPoints`))
  (if (`KismetSystemLibrary.DoesImplementInterface` OtherActor "/Game/Blueprints/EnemyObject.EnemyObject_C")
    (bind _asai_pawn_enemy (cast `/Game/Blueprints/AI_pawn_Enemy` OtherActor)
      (:`then`
        (`self.K2_DestroyActor` _asai_pawn_enemy)
        (bind _result (`/Engine/EditorBlueprintResources/StandardMacros.DecrementInt` _hitpoints)
          (:`  `
            (`self.Set DoorState` _result))))
      (:`CastFailed`
        (bind _asai_pawn_builder (cast `/Game/Blueprints/AI_pawn_Builder` OtherActor))
        (`self.K2_DestroyActor` _asai_pawn_builder)
        (bind _result_2 (`/Engine/EditorBlueprintResources/StandardMacros.IncrementInt` _hitpoints)
          (:`  `
            (`self.Set DoorState` _result_2)))))))

(fn `BuildWall`
  (bind _result (`/Engine/EditorBlueprintResources/StandardMacros.IncrementInt` (`self.HitPoints`))
    (:`  `
      (`self.Set DoorState` _result))))

(fn `removeMe`
  (returns (Remove :type Boolean))
  (return (`self.Dead`)))

(fn `Set DoorState`
  (params (HitPoints :type Integer))
  (bind _output_get (set `self.HitPoints` HitPoints))
  (switch `int` _output_get
    (:`Default`
      (`SceneComponent.SetVisibility` (`self.StaticMesh1`) true false)
      (`SceneComponent.SetVisibility` (`self.StaticMesh2`) true false)
      (`SceneComponent.SetVisibility` (`self.StaticMesh3`) true false)
      (`SceneComponent.SetVisibility` (`self.StaticMesh`) true false))
    (:`0`
      (bind _returnvalue (`GameplayStatics.GetActorOfClass` "/Game/Blueprints/AIGoalManager.AIGoalManager_C"))
      (set `self.Dead` true)
      (`/Game/Blueprints/AIGoalManager.UpdateGoals` _returnvalue))
    (:`1`
      (`SceneComponent.SetVisibility` (`self.StaticMesh1`) false false))
    (:`2`
      (`SceneComponent.SetVisibility` (`self.StaticMesh2`) false false))
    (:`3`
      (`SceneComponent.SetVisibility` (`self.StaticMesh3`) false false))))

(fn `UserConstructionScript`)