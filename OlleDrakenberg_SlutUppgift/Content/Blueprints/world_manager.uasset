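; World manager actor that spawns AI pawns and exposes the world transform of a gate.
; SpawnAI creates a pawn with its behavior tree at the given location, writes it into the Ai array, then increments an index and destroys the manager if that matches the array length.
; GetGateLocation returns the Gate's transform.
; The event graph is empty, so neither function is called within this Blueprint.
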(fn `GetGateLocation`
  (returns (NewParam :type "Transform Structure"))
  (return (`SceneComponent.K2_GetComponentToWorld` (`self.Gate`))))

(fn `Spawn AI`
  (params (spawnlocation :type "Transform Structure"))
  (locals (NewLocalVar_0 :type Integer :default 0))
  (bind _ai (`self.ai`))
  (bind _newlocalvar_0 (`local.NewLocalVar_0`))
  (bind _returnvalue (`AIBlueprintHelperLibrary.SpawnAIFromClass` "/Game/Blueprints/AI_pawn.AI_pawn_C" "/Game/Blueprints/AI_BehaviorTree.AI_BehaviorTree" (.location spawnlocation) (struct) false null))
  (`KismetArrayLibrary.Array_Set` _ai _newlocalvar_0 _returnvalue)
  (bind _result (`/Engine/EditorBlueprintResources/StandardMacros.IncrementInt` _newlocalvar_0)
    (:`  `
      (if (== _result (`KismetArrayLibrary.Array_Length` _ai))
        (`self.K2_DestroyActor`)))))

(fn `UserConstructionScript`)