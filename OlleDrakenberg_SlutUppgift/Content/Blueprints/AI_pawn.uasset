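; AI pawn that runs a Persuit, Attacking or Goal state each tick, with the Goal handler left empty.
; On BeginPlay it spawns its own Target actor and caches the player and an AIGoalManager, which is otherwise unused here.
; Persuit and Attacking teleport that Target to the player and adjust mesh mass scale per state.
; Persuit also raises floating-movement max speed to a multiple of the starting speed.
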(event `self.ReceiveBeginPlay`
  (set `self.StartSpeed` (`MovementComponent.GetMaxSpeed` (`self.MovementComponent`)))
  (set `self.Persuit` (* (`self.StartSpeed`) 2.2))
  (bind _returnvalue (`|SpawnActorFromClass` "/Game/Blueprints/Target.Target_C" (`self.GetTransform` self) "Undefined" "OverrideRootScale" null null))
  (set `self.aiTarget` _returnvalue)
  (bind _returnvalue_2 (`GameplayStatics.GetActorOfClass` "/Game/other/FirstPersonBP/Blueprints/Player_BP.Player_BP_C"))
  (set `self.PlayerRef` _returnvalue_2)
  (bind _returnvalue_3 (`GameplayStatics.GetActorOfClass` "/Game/Blueprints/AIGoalManager.AIGoalManager_C"))
  (set `self.AIManager` _returnvalue_3))

(event `self.ReceiveTick`
  (params (DeltaSeconds :type "Float (single-precision)"))
  (switch `/Game/Blueprints/AI/DataSheets/AiStates` (`self.Ai State`)
    (:`NewEnumerator4`
      (`self.HandlePersuit`))
    (:`NewEnumerator2`
      (`self.HandleAttack`))
    (:`NewEnumerator5`
      (`self.HandleGoal`))))

(fn `HandleAttack`
  (`self.SetTarget` (`self.K2_GetActorLocation` (`self.PlayerRef`)))
  (`self.ScaleAI`)
  (return))

(fn `HandleDeath`
  (`self.K2_DestroyActor`))

(fn `HandleGoal`
  (return))

(fn `HandlePersuit`
  (`self.ScaleAI`)
  (bind _asfloating_pawn_movement (cast `FloatingPawnMovement` (`self.MovementComponent`)))
  (set `FloatingPawnMovement.MaxSpeed` (`self.Persuit`) _asfloating_pawn_movement)
  (`self.SetTarget` (`self.K2_GetActorLocation` (`self.PlayerRef`))))

(fn `ScaleAI`
  (`/Engine/EditorBlueprintResources/StandardMacros.DoOnce` false :!label _label
    (:`Completed`
      (switch `/Game/Blueprints/AI/DataSheets/AiStates` (`self.Ai State`)
        (:`NewEnumerator4`
          (`PrimitiveComponent.SetMassScale` (`self.MeshComponent`) "None" 0.5)
          (goto _label :!via `Reset`))
        (:`NewEnumerator2`
          (`PrimitiveComponent.SetMassScale` (`self.MeshComponent`) "None" 1.5)
          (goto _label :!via `Reset`))
        (:`NewEnumerator5`
          (`PrimitiveComponent.SetMassScale` (`self.MeshComponent`) "None" 1.0)
          (goto _label :!via `Reset`))))))

(fn `SetAITarget`
  (switch `/Game/Blueprints/AI/DataSheets/AiStates` (`self.Ai State`)
    (:`NewEnumerator4`
      (`self.HandlePersuit`))
    (:`NewEnumerator2`
      (`self.HandleAttack`))
    (:`NewEnumerator5`
      (`self.HandleGoal`))))

(fn `SetTarget`
  (params (Target :type "Vector Structure"))
  (`self.K2_SetActorLocation` (`self.aiTarget`) Target false true)
  (return))

(fn `UserConstructionScript`)