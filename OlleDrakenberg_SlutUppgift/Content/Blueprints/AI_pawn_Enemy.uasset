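; Enemy AI pawn that reacts to the player through attack and pursuit overlap volumes, deferring much of its behavior to a parent class.
; Entering the attack area calls HandleAttack, which uses FlipFlop and DoOnce nodes around an in-range flag and red material feedback; leaving calls the parent's pursuit handler.
; Entering the pursuit area calls an empty HandleGoal, as its random-goal targeting from AIGoalManager is disconnected.
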(event `self.ReceiveBeginPlay`
  (`parent.ReceiveBeginPlay`)
  (bind _returnvalue (`GameplayStatics.GetActorOfClass` "/Game/other/FirstPersonBP/Blueprints/Player_BP.Player_BP_C"))
  (set `self.Player Ref` _returnvalue))

(event `self.AttackArea.OnComponentBeginOverlap`
  (params (OverlappedComponent :type "PrimitiveComponent Object Reference") (OtherActor :type "Actor Object Reference") (OtherComp :type "PrimitiveComponent Object Reference") (OtherBodyIndex :type Integer) (bFromSweep :type Boolean) (SweepResult :type "HitResult Structure (by ref)"))
  (cast `/Game/other/FirstPersonBP/Blueprints/Player_BP` OtherActor)
  (`self.HandleAttack`))

(event `self.AttackArea.OnComponentEndOverlap`
  (params (OverlappedComponent :type "PrimitiveComponent Object Reference") (OtherActor :type "Actor Object Reference") (OtherComp :type "PrimitiveComponent Object Reference") (OtherBodyIndex :type Integer))
  (cast `/Game/other/FirstPersonBP/Blueprints/Player_BP` OtherActor)
  (`self.HandlePersuit`))

(event `self.PresuitArea.OnComponentBeginOverlap`
  (params (OverlappedComponent :type "PrimitiveComponent Object Reference") (OtherActor :type "Actor Object Reference") (OtherComp :type "PrimitiveComponent Object Reference") (OtherBodyIndex :type Integer) (bFromSweep :type Boolean) (SweepResult :type "HitResult Structure (by ref)"))
  (cast `/Game/other/FirstPersonBP/Blueprints/Player_BP` OtherActor)
  (`self.HandleGoal`))

(event `self.PresuitArea.OnComponentEndOverlap`
  (params (OverlappedComponent :type "PrimitiveComponent Object Reference") (OtherActor :type "Actor Object Reference") (OtherComp :type "PrimitiveComponent Object Reference") (OtherBodyIndex :type Integer))
  (cast `/Game/other/FirstPersonBP/Blueprints/Player_BP` OtherActor))

(fn `HandleAttack`
  (bind _meshcomponent (`self.MeshComponent`))
  (`parent.HandleAttack`)
  (bind _isa (`/Engine/EditorBlueprintResources/StandardMacros.FlipFlop`)
    (:`A`
      (`/Engine/EditorBlueprintResources/StandardMacros.DoOnce` false :!label _label
        (:`Completed`
          (set `self.IsInAttackRange` true)
          (if _isa
            (`PrimitiveComponent.SetMaterial` _meshcomponent 0 "/Game/_material/Red.Red")
            (goto _label_2 :!via `Reset`)))))
    (:`B`
      (`/Engine/EditorBlueprintResources/StandardMacros.DoOnce` false :!label _label_2
        (:`Completed`
          (set `self.IsInAttackRange` false)
          (`PrimitiveComponent.SetMaterial` _meshcomponent 0 "/Game/other/Geometry/Meshes/CubeMaterial.CubeMaterial")
          (goto _label :!via `Reset`))))))

(fn `HandleGoal`)

(fn `HandlePersuit`
  (`parent.HandlePersuit`))

(fn `SetAITarget`
  (`parent.SetAITarget`))

(fn `UserConstructionScript`
  (`parent.UserConstructionScript`))