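; Spawner is a destructible wall or door with four meshes that loses hit points when a first-person projectile overlaps its sphere.
; SetDoorState stores the new value, hides one mesh at 3, 2 and 1, destroys the actor at 0, and otherwise shows all.
; Hits decrement MaxHitpoints, while BuildWall increments HitPoints.
; A CD flag blocks repeat damage, clearing two seconds after a subsequent hit.
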(event `self.ReceiveBeginPlay`
  (`SceneComponent.SetVisibility` (`self.StaticMesh1`) true false)
  (`SceneComponent.SetVisibility` (`self.StaticMesh2`) true false)
  (`SceneComponent.SetVisibility` (`self.StaticMesh3`) true false)
  (`SceneComponent.SetVisibility` (`self.StaticMesh`) true false)
  (set `self.HitPoints` (`self.MaxHitpoints`))
  (`SceneComponent.SetVisibility` (`self.StaticMesh`) true false))

(event `self.Sphere.OnComponentBeginOverlap`
  (params (OverlappedComponent :type "PrimitiveComponent Object Reference") (OtherActor :type "Actor Object Reference") (OtherComp :type "PrimitiveComponent Object Reference") (OtherBodyIndex :type Integer) (bFromSweep :type Boolean) (SweepResult :type "HitResult Structure (by ref)"))
  (cast `/Game/other/FirstPersonBP/Blueprints/FirstPersonProjectile` OtherActor)
  (if (`self.CD`)
    (`KismetSystemLibrary.Delay` 2.0)
    (set `self.CD` false)
    (else
      (bind _result (`/Engine/EditorBlueprintResources/StandardMacros.DecrementInt` (`self.MaxHitpoints`))
        (:`  `
          (`self.Set DoorState` _result)
          (set `self.CD` true))))))

(fn `BuildWall`
  (bind _result (`/Engine/EditorBlueprintResources/StandardMacros.IncrementInt` (`self.HitPoints`))
    (:`  `
      (`self.Set DoorState` _result))))

(fn `Set DoorState`
  (params (HitPoints :type Integer))
  (bind _output_get (set `self.HitPoints` HitPoints))
  (switch `int` _output_get
    (:`Default`
      (`SceneComponent.SetVisibility` (`self.StaticMesh1`) true false)
      (`SceneComponent.SetVisibility` (`self.StaticMesh2`) true false)
      (`SceneComponent.SetVisibility` (`self.StaticMesh3`) true false)
      (`SceneComponent.SetVisibility` (`self.StaticMesh`) true false))
    (:`0`
      (`self.K2_DestroyActor`))
    (:`1`
      (`SceneComponent.SetVisibility` (`self.StaticMesh1`) false false))
    (:`2`
      (`SceneComponent.SetVisibility` (`self.StaticMesh2`) false false))
    (:`3`
      (`SceneComponent.SetVisibility` (`self.StaticMesh3`) false false))))

(fn `UserConstructionScript`)