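; AI goal manager that builds the level's set of AI goals once at BeginPlay through UpdateGoals.
; It gathers every actor implementing the GoalObject interface into PotentialGoals, destroying any Door whose RemoveMe returns true.
; Each remaining actor gets an AIGoalBP spawned at its location and stored in GoalBP at the same index.
; GoalHandeler is an empty stub.
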(event `self.ReceiveBeginPlay`
  (`self.UpdateGoals`))

(fn `Goal Handeler`
  (params (Pawn :type "/Game/Blueprints/AI_pawn Object Reference")))

(fn `UpdateGoals`
  (bind _outactors (`GameplayStatics.GetAllActorsWithInterface` "/Game/Blueprints/GoalObject.GoalObject_C"))
  (bind _output_get (set `self.PotentialGoals` _outactors))
  (for (_array_element _array_index) _output_get
    (bind _asdoor (cast `/Game/Blueprints/Door` _array_element)
      (:`then`
        (bind _remove (`/Game/Blueprints/Door.removeMe` _asdoor))
        (if _remove
          (`self.K2_DestroyActor` _asdoor)
          (else
            (bind _returnvalue (`|SpawnActorFromClass` "/Game/Blueprints/AIGoalBP.AIGoalBP_C" (`KismetMathLibrary.Conv_VectorToTransform` (`self.K2_GetActorLocation` _array_element)) "AlwaysSpawn" "OverrideRootScale" null null :!label _label))
            (`KismetArrayLibrary.Array_Set` (`self.GoalBP`) _array_index _returnvalue))))
      (:`CastFailed`
        (goto _label)))))

(fn `UserConstructionScript`)